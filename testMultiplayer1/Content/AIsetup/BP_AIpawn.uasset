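; BP_AIpawn is an AI pawn that moves between two hardcoded locations on cue from the gameplay game mode.
; On BeginPlay it casts to GM_GameplayLevel and binds to its MoveAI event dispatcher, printing a failure message if the cast fails.
; Each call flips a FlipFlop to alternate the AI MoveTo target, keeping the capsule's current height.
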(event Custom|MoveAI_Event
  (bind _self self)
  (bind _capsulecomponent (Variables|Collision|GetCapsuleComponent))
  (bind _returnvalue (Transformation|GetWorldLocation _capsulecomponent))
  (bind _z (Math|Vector|BreakVector _returnvalue))
  (Utilities|FlowControl|FlipFlop
    (:A
      (AI|AIMoveTo _self (Math|Vector|MakeVector -3.7e+02 -6.5e+02 _z) 0 5.0 false))
    (:B
      (AI|AIMoveTo _self (Math|Vector|MakeVector -7.1e+02 -3.8e+02 _z) 0 5.0 false))))

(event EventBeginPlay
  (bind _asgm_gameplay_level (Utilities|Casting|CastToGM_GameplayLevel (Game|GetGameMode))
    (:then
      (bind _output_get (Variables|Default|SetAs%20GM%20Gameplay%20Level _asgm_gameplay_level))
      (EventDispatchers|BindEventtoMoveAI _output_get (delegate Custom|MoveAI_Event)))
    (:CastFailed
      (Development|PrintString "ai fail"))))

(fn ConstructionScript)