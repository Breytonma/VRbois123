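; PlayFab game instance that handles player account signup, email login and password recovery.
; Init sets the PlayFab title ID, and Signup, Login and ForgotPassword events each send a client request.
; Successful signup or login opens the gameplay level after a short delay, while recovery prints a confirmation.
; Only signup binds a failure handler, which prints the error, and an unconnected JoinLobby call never runs.
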(event Custom|Forgot%20Password
  (params (Email :type String))
  ;[1 0.4001 0.3852] Forgot Password
  (|SendAccountRecoveryEmail (Utilities|Struct|MakeClientSendAccountRecoveryEmailRequest 0 Email) (delegate Custom|On%20Recovery%20Email%20Success)))

(event Custom|On%20Recovery%20Email%20Success
  (params (result :type Client%20Send%20Account%20Recovery%20Email%20Result%20Structure) (customData :type Object%20Object%20Reference))
  ;[1 0.4001 0.3852] Forgot Password
  (Development|PrintString "Recovery Email Has been sent" true true "(R=0.000000,G=1.000000,B=0.078017,A=1.000000)" 1e+01))

(event Custom|Signup
  (params (Username :type String) (Email :type String) (Password :type String))
  ;[1 0.639 0.2524] Signup
  (|RegisterPlayFabUser (Utilities|Struct|MakeClientRegisterPlayFabUserRequest 0 Username Email "" 0 Password "" false Username) (delegate Custom|OnRegisterSuccess) (delegate Custom|OnFail)))

(event Custom|Login
  (params (Email :type String) (Password :type String))
  ;[0.3039 1 0.257] Login
  (|LoginwithEmailAddress (Utilities|Struct|MakeClientLoginWithEmailAddressRequest 0 Email 0 Password) (delegate Custom|OnLoginSuccess)))

(event Custom|OnFail
  (params (error :type Play%20Fab%20Error%20Structure) (customData :type Object%20Object%20Reference))
  ;[1 0.639 0.2524] Signup
  (Development|PrintString (Utilities|String|Append (.errorname error) ": " (.errormessage error) "(" (.errordetails error) ")") true true "(R=1.000000,G=0.080382,B=0.000000,A=1.000000)" 1e+01))

(event Custom|OnRegisterSuccess
  (params (result :type Client%20Register%20Play%20Fab%20User%20Result%20Structure) (customData :type Object%20Object%20Reference))
  ;[1 0.639 0.2524] Signup
  (Utilities|FlowControl|Delay 1.0)
  (Game|OpenLevel(byObjectReference) "/Game/Sessions/levels/Gameplay_Level.Gameplay_Level"))

(event Custom|OnLoginSuccess
  (params (result :type Client%20Login%20Result%20Structure) (customData :type Object%20Object%20Reference))
  ;[0.3039 1 0.257] Login
  (Utilities|FlowControl|Delay 1.0)
  (Game|OpenLevel(byObjectReference) "/Game/Sessions/levels/Gameplay_Level.Gameplay_Level"))

(event EventInit
  (Class|PlayFabUtilities|SetPlayFabSettings (Variables|Default|GetPlayFab_GameID)))